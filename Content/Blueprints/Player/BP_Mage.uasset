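; BP_Mage is the player character, with camera-relative movement, mesh rotation smoothed toward input, jump, dash and a rope grapple.
; F launches a dash on a cooldown; jump has an IsDashing momentum-launch branch, though the dash never sets that flag.
; Right mouse plays the grapple montage; ThrowRope line-traces for "Anchor"-tagged actors, then a timeline pulls the character along a visible cable.
; OnPlayerDeath shows the game-over widget and pauses.
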(event `self.ReceiveBeginPlay`
  ;[0.03125 0.03125 0.03125] Input Setup
  (`EnhancedInputSubsystemInterface.AddMappingContext` (pcsubsystem `EnhancedInputLocalPlayerSubsystem` (`GameplayStatics.GetPlayerController` 0)) "/Game/Inputs/IM_MageContext.IM_MageContext" 0 (struct)))

(event `InputAxisKey|MouseX`
  (params (AxisValue :type "Float (single-precision)"))
  ;[1 1 1] Look
  (`self.AddControllerYawInput` AxisValue))

(event `InputAxisKey|MouseY`
  (params (AxisValue :type "Float (single-precision)"))
  ;[1 1 1] Look
  (bind _result (`/Engine/EditorBlueprintResources/StandardMacros.NegateFloat` AxisValue)
    (:`  `
      (`self.AddControllerPitchInput` _result))))

(event `EnhancedInput|/Game/Inputs/IA_Move`
  (params (ActionValue :type "Vector2D Structure") (ElapsedSeconds :type "Float (double-precision)") (TriggeredSeconds :type "Float (double-precision)") (InputAction :type "InputAction Object Reference" :default "/Game/Inputs/IA_Move.IA_Move"))
  (bind _camera (`self.Camera`))
  (bind (_returnvalue_x _returnvalue_y) (`KismetMathLibrary.BreakVector` (`SceneComponent.GetForwardVector` _camera)))
  ;[0.04534 0.0707 0.1198] Movement
  (:`Triggered`
    (`self.AddMovementInput` (+ (* ActionValue_X (`KismetMathLibrary.Normal` (`KismetMathLibrary.MakeVector` _returnvalue_x _returnvalue_y))) (* ActionValue_Y (`SceneComponent.GetRightVector` _camera))))))

(event `self.ReceiveTick`
  (params (DeltaSeconds :type "Float (single-precision)"))
  (bind _mesh (`self.Mesh`))
  (bind _returnvalue (`PawnMovementComponent.GetLastInputVector` (`self.CharacterMovement`)))
  ;[0.04001 0.05217 0.1302] PlayerRotation
  (`|ExecutionSequence`
    (:`then_0`
      (if (> (`KismetMathLibrary.VSize` _returnvalue) 0.0)
        (bind _result (`/Engine/EditorBlueprintResources/StandardMacros.NegateFloat` (.x _returnvalue))
          (:`  `
            (set `self.TargetRotation` (`KismetMathLibrary.MakeRotFromX` (`KismetMathLibrary.MakeVector` (.y _returnvalue) _result (.z _returnvalue))))))))
    (:`then_1`
      (`SceneComponent.K2_SetWorldRotation` _mesh (`KismetMathLibrary.RLerp` (`SceneComponent.K2_GetComponentRotation` _mesh) (`self.TargetRotation`) (* DeltaSeconds (`self.RotationSpeed`)) true) false false))))

(event `/Game/Blueprints/Player/BPI_PlayerAction.OnPlayerDeath`
  (bind _returnvalue (`GameplayStatics.GetPlayerController` 0))
  ;[0.02604 0.02428 0.02428] Trigger GameOver Screen on Death
  (bind _returnvalue_2 (`|CreateWidget` "/Game/Blueprints/UI/WBP_GameOver.WBP_GameOver_C"))
  (`UserWidget.AddToViewport` _returnvalue_2 0)
  (set `PlayerController.bShowMouseCursor` true _returnvalue)
  (`WidgetBlueprintLibrary.SetInputMode_UIOnlyEx` _returnvalue null)
  (`GameplayStatics.SetGamePaused` true))

(event `EnhancedInput|/Game/Inputs/IA_Jump`
  (params (ActionValue :type Boolean) (ElapsedSeconds :type "Float (double-precision)") (TriggeredSeconds :type "Float (double-precision)") (InputAction :type "InputAction Object Reference" :default "/Game/Inputs/IA_Jump.IA_Jump"))
  ;[0.04167 0.00433 0.005159] Jump ( When you dash and jump you gain momentum)
  (:`Started`
    (if (`self.IsDashing`)
      (`MovementComponent.StopMovementImmediately` (`self.CharacterMovement`))
      (`self.LaunchCharacter` (`KismetMathLibrary.MakeVector` (* (.x (`self.GetVelocity`)) 1.2) (* (.y (`self.GetVelocity`)) 1.2) 800.0) true true)
      (set `self.IsDashing` true)
      (`KismetSystemLibrary.Delay` 2.0)
      (set `self.IsDashing` false)
      (else
        (`self.Jump`)
        (`GameplayStatics.PlaySound2D` "/Game/GameSounds/SoundEffects/freesound_community-video-game-jump-soundeffect-37532.freesound_community-video-game-jump-soundeffect-37532" 0.3 1.0 0.0 null null)
        (`NiagaraFunctionLibrary.SpawnSystemAttached` "/Game/Particles/JumpParticles.JumpParticles" (`self.Mesh`) "None" (0.0 0.0 0.0) (struct) "SnapToTarget" true)))))

(event `Key|F`
  (params (Key :type "Key Structure"))
  ;[0.01681 0.001821 0.002125] Dash
  (:`Pressed`
    (`NiagaraFunctionLibrary.SpawnSystemAttached` "/Game/Particles/DashParticles.DashParticles" (`self.Mesh`) "spine" (0.0 0.0 0.0) (struct) "SnapToTarget" true)
    (if (not (`self.HasDashed`))
      (`MovementComponent.StopMovementImmediately` (`self.CharacterMovement`))
      (`self.LaunchCharacter` (* (`KismetMathLibrary.MakeVector` (.x (`SceneComponent.GetForwardVector` (`self.Camera`))) (.y (`SceneComponent.GetForwardVector` (`self.Camera`)))) (`self.DashSpeed`)) true true)
      (`GameplayStatics.PlaySound2D` "/Game/GameSounds/Music/DashSound.DashSound" 1.0 (`KismetMathLibrary.RandomFloatInRange` 0.85 1.15) 0.0 null null)
      (set `self.HasDashed` true)
      (`KismetSystemLibrary.Delay` 2.0)
      (set `self.HasDashed` false))))

(event `ThrowRope`
  (bind _returnvalue (`self.K2_GetActorLocation`))
  (bind _cable (`self.Cable`))
  ;[0.006995 0.000911 0.000911] Line trace for rope pulling and throw rope event triggering
  (set `self.isGrappling` true)
  (bind (_outhit _returnvalue_2) (`KismetSystemLibrary.LineTraceSingle` _returnvalue (+ _returnvalue (* (`KismetMathLibrary.GetForwardVector` (`self.GetControlRotation`)) (`self.RopeLength`))) "TraceTypeQuery1"))
  (if _returnvalue_2
    (bind (_bblockinghit _binitialoverlap _time _distance _location _impactpoint _normal _impactnormal _physmat _hitactor _hitcomponent) (`GameplayStatics.BreakHitResult` _outhit))
    (if (`self.ActorHasTag` _hitactor "Anchor")
      (set `self.EndLocationGrapple` _impactpoint)
      (`SceneComponent.SetVisibility` _cable true false)
      (`CableComponent.SetAttachEndToComponent` _cable _hitcomponent "None")
      (set `self.StartLocationGrapple` (`self.K2_GetActorLocation`))
      (`CharacterMovementComponent.SetMovementMode` (`self.CharacterMovement`) "MOVE_None" 0)
      (`GameplayStatics.PlaySound2D` "/Game/GameSounds/SoundEffects/floraphonic-stretch-rubber-rope-foley-2-209715_dYnYMKiU.floraphonic-stretch-rubber-rope-foley-2-209715_dYnYMKiU" 0.5 1.0 0.0 null null false)
      (bind (_direction _roapfloat) (`Timeline|Grapple` :!via `PlayFromStart`)
        (:`Update`
          (`self.K2_SetActorLocation` (`KismetMathLibrary.VLerp` (`self.StartLocationGrapple`) (`self.EndLocationGrapple`) _roapfloat) true)
          (set `self.isGrappling` false))
        (:`Finished`
          (`CharacterMovementComponent.SetMovementMode` (`self.CharacterMovement`) "MOVE_Falling" 0)
          (`SceneComponent.SetVisibility` (`self.Cable`) false false))))))

(event `Key|RightMouseButton`
  (params (Key :type "Key Structure"))
  ;[0.006995 0.000911 0.000911] Line trace for rope pulling and throw rope event triggering
  (:`Pressed`
    (`self.PlayAnimMontage` "/Game/PlayerModels-Animations/PlayerAnimations/GrapplingHook.GrapplingHook")))

(fn `UserConstructionScript`)