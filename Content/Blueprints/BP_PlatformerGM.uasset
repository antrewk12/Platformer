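; BP_PlatformerGM is the platformer game mode that tracks score and elapsed time.
; On BeginPlay it creates a WBP_HUD widget, stores a reference and adds it to the viewport.
; AddScore accumulates points and pushes the new total to the HUD, while Tick adds delta seconds to a timer whenever TimeRunning is set.
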(event `self.ReceiveBeginPlay`
  ;[0.06771 0.06771 0.06771] Create the widget reference to hud
  (bind _returnvalue (`|CreateWidget` "/Game/Blueprints/UI/WBP_HUD.WBP_HUD_C"))
  (bind _output_get (set `self.ScoreWidget Reference` _returnvalue))
  (`UserWidget.AddToViewport` _output_get 0))

(event `AddScore`
  (params (Amount :type Integer))
  ;[1 1 1] Hook up the custom event to the event of the HUD WIDGET
  (bind _output_get (set `self.Score` (+ Amount (`self.Score`))))
  (`/Game/Blueprints/UI/WBP_HUD.UpdateScore` (`self.ScoreWidget Reference`) _output_get))

(event `self.ReceiveTick`
  (params (DeltaSeconds :type "Float (single-precision)"))
  ;[1 1 1] Timer clock
  (if (`self.TimeRunning`)
    (set `self.Time` (+ (`GameplayStatics.GetWorldDeltaSeconds`) (`self.Time`)))))

(fn `UserConstructionScript`)